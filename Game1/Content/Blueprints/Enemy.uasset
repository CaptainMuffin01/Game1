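; Enemy Blueprint that tracks health, takes damage and removes itself on death.
; The DamageHealth event subtracts DamageAmount from CurrentHealth.
; Tick polls health through a 0.2-second Delay rather than checking when damage lands, and calls ActorDeath at zero or below to destroy the actor.
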(event `self.ReceiveTick`
  (params (DeltaSeconds :type "Float (single-precision)"))
  ;[1 1 1] EmenyDamage
  (`KismetSystemLibrary.Delay` 0.2)
  (if (<= (`self.Current health`) 0.0)
    (`self.ActorDeath`)))

(event `ActorDeath`
  ;[1 1 1] EmenyDamage
  (`self.K2_DestroyActor`))

(event `DamageHealth`
  ;[1 1 1] EmenyDamage
  (set `self.Current health` (- (`self.Current health`) (`self.DamageAmount`))))

(fn `UserConstructionScript`)